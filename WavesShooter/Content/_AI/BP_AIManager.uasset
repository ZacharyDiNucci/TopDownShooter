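; AI wave manager that runs the enemy waves across two levels, opening each behind a brief loading screen.
; Each wave follows a countdown widget, then spawns melee and random ranged enemies at navigable points around AISpawnLocation actors, with ranged ones arriving sooner and likelier in level two.
; Kill events empty the tracked enemy list, triggering a larger next wave.
; After wave ten, it advances the GameInstance level or shows the Win screen.
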(event `self.ReceiveBeginPlay`
  (bind _asstore_vars_1 (cast `/Game/StoreVars1` (`GameplayStatics.GetGameInstance`)))
  (bind _output_get (set `self.Level` (`/Game/StoreVars1.level` _asstore_vars_1)))
  (if (== _output_get 1)
    (bind _returnvalue (`|CreateWidget` "/Game/LoadingScreen1.LoadingScreen1_C"))
    (`UserWidget.AddToViewport` _returnvalue 0)
    (`KismetSystemLibrary.Delay` 0.9)
    (else
      (bind _returnvalue_2 (`|CreateWidget` "/Game/LoadingScreen2.LoadingScreen2_C"))
      (`UserWidget.AddToViewport` _returnvalue_2 0)
      (`KismetSystemLibrary.Delay` 0.9)))
  (`WidgetLayoutLibrary.RemoveAllWidgets`)
  (`|ExecutionSequence`
    (:`then_0`
      (`KismetSystemLibrary.Delay` 0.2)
      (bind _outactors (`GameplayStatics.GetAllActorsOfClass` "/Game/_AI/AISpawnLocation.AISpawnLocation_C"))
      (for _array_element _outactors
        (`KismetArrayLibrary.Array_Add` (`self.Spawners`) _array_element)))
    (:`then_1`
      (`KismetSystemLibrary.Delay` 2.0)
      (`self.CountdownWave`))))

(event `CountdownWave`
  (bind _returnvalue (`GameplayStatics.GetPlayerController` 0))
  (bind _timeuntilwavebegins (`self.TimeUntilWaveBegins`))
  (if (== (`self.WaveAmount`) 10)
    (if (== (`self.Level`) 1)
      (if (not (`self.resetWave`))
        (`/Game/Countdown.UpdateLoadTimer` (`self.W_Countdown`) 10)
        (bind _asstore_vars_1 (cast `/Game/StoreVars1` (`GameplayStatics.GetGameInstance`)))
        (set `/Game/StoreVars1.level` 2 _asstore_vars_1))
      (else
        (bind _returnvalue_2 (`|CreateWidget` "/Game/Win.Win_C" (`GameplayStatics.GetPlayerController` 0)))
        (bind _output_get (set `self.Win` _returnvalue_2))
        (`UserWidget.AddToViewport` _output_get 0)
        (`WidgetBlueprintLibrary.SetInputMode_GameOnly` _returnvalue)
        (set `PlayerController.bShowMouseCursor` false _returnvalue)))
    (else
      (set `self.WaveAmount` (+ (`self.WaveAmount`) 1))
      (`self.W_Countdown`
        (:`then`
          _)
        (:`else`
          (bind _returnvalue_3 (`|CreateWidget` "/Game/Countdown.Countdown_C" (`GameplayStatics.GetPlayerController` 0)))
          (bind _output_get_2 (set `self.W_Countdown` _returnvalue_3))
          (`UserWidget.AddToViewport` _output_get_2 0)))
      (`/Game/Countdown.UpdateWaveTImer` (`self.W_Countdown`) _timeuntilwavebegins)
      (`KismetSystemLibrary.K2_SetTimer` null "SpawnNextWave" (`KismetMathLibrary.Conv_IntToDouble` _timeuntilwavebegins))
      (`/Game/Countdown.UpdateWaveCount` (`self.W_Countdown`) (`self.WaveAmount`)))))

(event `SpawnNextWave`
  (bind _spawners (`self.Spawners`))
  (bind _spawners_2 (`self.Spawners`))
  (bind _spawners_3 (`self.Spawners`))
  (bind _spawners_4 (`self.Spawners`))
  (bind _spawners_5 (`self.Spawners`))
  (bind _spawners_6 (`self.Spawners`))
  (if (<= (`self.Level`) 1)
    (if (<= (`self.WaveAmount`) 4)
      (for _ (range 1 (+ (`self.EnemiesToSpawn`) 1))
        (bind _returnvalue (`|SpawnActorFromClass` "/Game/_AI/Enemy_Melee.Enemy_Melee_C" (`KismetMathLibrary.MakeTransform` (+ (`NavigationSystemV1.K2_GetRandomReachablePointInRadius` (`self.K2_GetActorLocation` (`|GetArrayItem` _spawners_2 (`KismetMathLibrary.RandomIntegerInRange` 0 (- (`KismetArrayLibrary.Array_Length` _spawners_2) 1)))) 200.0 null null) (0.0 0.0 88.0))) "AdjustIfPossibleButAlwaysSpawn" "OverrideRootScale" null null))
        (`self.enemiesSpawned` _returnvalue))
      (else
        (for _ (range 1 (+ (`self.EnemiesToSpawn`) 1))
          (if (== (`KismetMathLibrary.RandomIntegerInRange` 1 4) 4)
            (bind _returnvalue_2 (`|SpawnActorFromClass` "/Game/_AI/Enemy_Ranged.Enemy_Ranged_C" (`KismetMathLibrary.MakeTransform` (+ (`NavigationSystemV1.K2_GetRandomReachablePointInRadius` (`self.K2_GetActorLocation` (`|GetArrayItem` _spawners_4 (`KismetMathLibrary.RandomIntegerInRange` 0 (- (`KismetArrayLibrary.Array_Length` _spawners_4) 1)))) 200.0 null null) (0.0 0.0 88.0))) "AdjustIfPossibleButAlwaysSpawn" "OverrideRootScale" null null))
            (`self.enemiesSpawned` _returnvalue_2)
            (else
              (bind _returnvalue_3 (`|SpawnActorFromClass` "/Game/_AI/Enemy_Melee.Enemy_Melee_C" (`KismetMathLibrary.MakeTransform` (+ (`NavigationSystemV1.K2_GetRandomReachablePointInRadius` (`self.K2_GetActorLocation` (`|GetArrayItem` _spawners_3 (`KismetMathLibrary.RandomIntegerInRange` 0 (- (`KismetArrayLibrary.Array_Length` _spawners_3) 1)))) 200.0 null null) (0.0 0.0 88.0))) "AdjustIfPossibleButAlwaysSpawn" "OverrideRootScale" null null))
              (`self.enemiesSpawned` _returnvalue_3))))))
    (elif (<= (`self.WaveAmount`) 0)
      (for _ (range 1 (+ (`self.EnemiesToSpawn`) 1))
        (bind _returnvalue_4 (`|SpawnActorFromClass` "/Game/_AI/Enemy_Melee.Enemy_Melee_C" (`KismetMathLibrary.MakeTransform` (+ (`NavigationSystemV1.K2_GetRandomReachablePointInRadius` (`self.K2_GetActorLocation` (`|GetArrayItem` _spawners_6 (`KismetMathLibrary.RandomIntegerInRange` 0 (- (`KismetArrayLibrary.Array_Length` _spawners_6) 1)))) 200.0 null null) (0.0 0.0 88.0))) "AdjustIfPossibleButAlwaysSpawn" "OverrideRootScale" null null))
        (`self.enemiesSpawned` _returnvalue_4))
      (else
        (for _ (range 1 (+ (`self.EnemiesToSpawn`) 1))
          (if (<= (`KismetMathLibrary.RandomIntegerInRange` 1 8) 3)
            (bind _returnvalue_5 (`|SpawnActorFromClass` "/Game/_AI/Enemy_Ranged.Enemy_Ranged_C" (`KismetMathLibrary.MakeTransform` (+ (`NavigationSystemV1.K2_GetRandomReachablePointInRadius` (`self.K2_GetActorLocation` (`|GetArrayItem` _spawners_5 (`KismetMathLibrary.RandomIntegerInRange` 0 (- (`KismetArrayLibrary.Array_Length` _spawners_5) 1)))) 200.0 null null) (0.0 0.0 88.0))) "AdjustIfPossibleButAlwaysSpawn" "OverrideRootScale" null null))
            (`self.enemiesSpawned` _returnvalue_5)
            (else
              (bind _returnvalue_6 (`|SpawnActorFromClass` "/Game/_AI/Enemy_Melee.Enemy_Melee_C" (`KismetMathLibrary.MakeTransform` (+ (`NavigationSystemV1.K2_GetRandomReachablePointInRadius` (`self.K2_GetActorLocation` (`|GetArrayItem` _spawners (`KismetMathLibrary.RandomIntegerInRange` 0 (- (`KismetArrayLibrary.Array_Length` _spawners) 1)))) 200.0 null null) (0.0 0.0 88.0))) "AdjustIfPossibleButAlwaysSpawn" "OverrideRootScale" null null))
              (`self.enemiesSpawned` _returnvalue_6))))))))

(fn `enemiesSpawned`
  (params (Enemy :type "/Game/_AI/BP_Enemy_Base Object Reference"))
  (`KismetArrayLibrary.Array_Add` (`self.Enemies`) Enemy)
  (add `/Game/_AI/BP_Enemy_Base.OnKilled` Enemy (`|CreateDelegate` :!event `EnemyKilled`)))

(fn `EnemyKilled`
  (params (Enemy :type "/Game/_AI/BP_Enemy_Base Object Reference"))
  (`KismetArrayLibrary.Array_RemoveItem` (`self.Enemies`) Enemy)
  (if (<= (`KismetArrayLibrary.Array_Length` (`self.Enemies`)) 0)
    (if (== (`self.Level`) 1)
      (set `self.EnemiesToSpawn` (+ (`self.EnemiesToSpawn`) 2))
      (`self.CountdownWave`)
      (elif (`self.resetWave`)
        (set `self.EnemiesToSpawn` (+ (`self.EnemiesToSpawn`) 4))
        (`self.CountdownWave`)
        (else
          (set `self.EnemiesToSpawn` 10)
          (set `self.resetWave` true)
          (`self.EnemyKilled` null))))))

(fn `UserConstructionScript`)