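; Base enemy character Blueprint that chases a target, attacks as either melee or ranged, and awards player score when killed.
; MoveToPlayer drives AIMoveTo; melee reaches the target and applies sphere-overlap damage on a montage notify, while ranged fires projectiles when ShootOverlap triggers.
; Attacks call MoveToPlayer again to continue the chase.
; AnyDamage triggers Death, which notifies OnKilled, sometimes drops a health pack, and destroys the actor.
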(event `self.ReceiveAnyDamage`
  (params (Damage :type "Float (single-precision)") (DamageType :type "DamageType Object Reference") (InstigatedBy :type "Controller Object Reference") (DamageCauser :type "Actor Object Reference"))
  (if (not (`self.Dead`))
    (set `self.Health` (- (`self.Health`) Damage))
    (if (<= (`self.Health`) 1.0)
      (`self.Death`)
      (`self.UpdatePlayerScore`))))

(event `Death`
  (if (not (`self.Dead`))
    (set `self.Dead` true)
    (`self.OnKilled` self)
    (`CharacterMovementComponent.DisableMovement` (`self.CharacterMovement`))
    (`PrimitiveComponent.SetCollisionEnabled` (`self.CapsuleComponent`) "NoCollision")
    (`SkeletalMeshComponent.PlayAnimation` (`self.Mesh`) null false)
    (`KismetSystemLibrary.Delay` 0.1)
    (if (== (`KismetMathLibrary.RandomIntegerInRange` 1 4) 4)
      (`|SpawnActorFromClass` "/Game/Materials/BP_HealthPack.BP_HealthPack_C" (`KismetMathLibrary.MakeTransform` (`SceneComponent.K2_GetComponentLocation` (`self.Mesh`))) "Undefined" "OverrideRootScale" null null)
      (`self.K2_DestroyActor`)
      (`AddComponent|NODE_AddParticleSystemComponent-0`)
      (else
        (`self.K2_DestroyActor`)
        (`AddComponent|NODE_AddParticleSystemComponent-1`)))))

(event `MoveToPlayer`
  (params (Target :type "Pawn Object Reference"))
  (if (`self.Melee`)
    (set `self.Player Target` Target)
    (`|AIMoveTo` self (0.0 0.0 0.0) Target 80.0
      (:`OnSuccess`
        (`self.Attack`)))
    (else
      (set `self.Player Target` Target)
      (`|AIMoveTo` self (0.0 0.0 0.0) Target 200.0
        (:`then`
          (`KismetSystemLibrary.K2_SetTimer` null "" 1.0 true)
          (add `PrimitiveComponent.OnComponentBeginOverlap` (`self.ShootOverlap`) (delegate `OnComponentBeginOverlap_Event_0`)))))))

(event `OnComponentBeginOverlap_Event_0`
  (params (OverlappedComponent :type "PrimitiveComponent Object Reference") (OtherActor :type "Actor Object Reference") (OtherComp :type "PrimitiveComponent Object Reference") (OtherBodyIndex :type Integer) (bFromSweep :type Boolean) (SweepResult :type "HitResult Structure (by ref)"))
  (if (not (`self.Melee`))
    (`self.Attack`)))

(event `Attack`
  (if (`self.Melee`)
    (`|PlayMontage` (`self.Mesh`) (`self.AttackMontage`)
      (:`OnNotifyBegin`
        (bind (_outactors _returnvalue) (`KismetSystemLibrary.SphereOverlapActors` (`SceneComponent.K2_GetComponentLocation` (`self.attackPoint`)) 80.0 (`|MakeArray` "ObjectTypeQuery10" :!type "EObjectTypeQuery Enum") "/Game/ThirdPersonBP/Blueprints/ThirdPersonCharacter.ThirdPersonCharacter_C"))
        (if _returnvalue
          (for _array_element _outactors
            (`GameplayStatics.ApplyDamage` _array_element (`self.Base Damage`) null self)
            (`KismetSystemLibrary.Delay` 1.0)
            (`self.MoveToPlayer` (`self.Player Target`)))
          (else
            (`self.MoveToPlayer` (`self.Player Target`))))))
    (else
      (`|SpawnActorFromClass` "/Game/Materials/BP_shotEnemy.BP_shotEnemy_C" (`KismetMathLibrary.MakeTransform` (`SceneComponent.K2_GetComponentLocation` (`self.Spawner`)) (`KismetMathLibrary.Conv_VectorToRotator` (`self.GetActorForwardVector`)) (0.6 0.07 0.0425)) "Undefined" "OverrideRootScale" null null)
      (`KismetSystemLibrary.Delay` 1.5)
      (`self.MoveToPlayer` (`self.Player Target`)))))

(event `UpdatePlayerScore`
  (bind _asthird_person_character (cast `/Game/ThirdPersonBP/Blueprints/ThirdPersonCharacter` (`GameplayStatics.GetPlayerCharacter` 0)))
  (`/Game/ThirdPersonBP/Blueprints/ThirdPersonCharacter.UpdateScore` _asthird_person_character (`self.ScoreValue`)))

(fn `UserConstructionScript`)