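; BP_HealthPack is a pickup that restores 25 health to the player character, capped at 100.
; On overlap it checks that the other actor's class is exactly ThirdPersonCharacter, then changes Health on player 0's character rather than on the overlapping actor.
; It pushes the new value to that character's PlayerUI and destroys itself after a brief delay.
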(event `self.ReceiveActorBeginOverlap`
  (params (OtherActor :type "Actor Object Reference"))
  (if (== (`GameplayStatics.GetObjectClass` OtherActor) "/Game/ThirdPersonBP/Blueprints/ThirdPersonCharacter.ThirdPersonCharacter_C")
    (bind _asthird_person_character (cast `/Game/ThirdPersonBP/Blueprints/ThirdPersonCharacter` (`GameplayStatics.GetPlayerCharacter` 0)))
    (bind _output_get (set `/Game/ThirdPersonBP/Blueprints/ThirdPersonCharacter.Health` (+ (`/Game/ThirdPersonBP/Blueprints/ThirdPersonCharacter.Health` _asthird_person_character) 25.0) _asthird_person_character))
    (if (<= _output_get 100.0)
      (`/Game/PlayerUI.UpdateHealth` (`/Game/ThirdPersonBP/Blueprints/ThirdPersonCharacter.Player UI` _asthird_person_character) _output_get)
      (`KismetSystemLibrary.Delay` 0.1)
      (`self.K2_DestroyActor`)
      (else
        (bind _asthird_person_character_2 (cast `/Game/ThirdPersonBP/Blueprints/ThirdPersonCharacter` (`GameplayStatics.GetPlayerCharacter` 0)))
        (bind _output_get_2 (set `/Game/ThirdPersonBP/Blueprints/ThirdPersonCharacter.Health` 100.0 _asthird_person_character_2))
        (`/Game/PlayerUI.UpdateHealth` (`/Game/ThirdPersonBP/Blueprints/ThirdPersonCharacter.Player UI` _asthird_person_character_2) _output_get_2)
        (`KismetSystemLibrary.Delay` 0.1)
        (`self.K2_DestroyActor`)))))

(fn `UserConstructionScript`)